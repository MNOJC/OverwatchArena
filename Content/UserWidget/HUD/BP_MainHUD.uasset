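; Main HUD Blueprint that puts the crosshair and a toggleable scope overlay on screen.
; On BeginPlay it creates the crosshair widget and adds it to the viewport, where it stays while the scope is shown.
; The Show/HideScope event flips a Scope flag, creating a fresh scope widget each time it turns on and removing the stored one when it turns off.
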(event `self.ReceiveBeginPlay`
  (bind _returnvalue (`|CreateWidget` "/Game/UserWidget/WBP_Crossair.WBP_Crossair_C"))
  (`UserWidget.AddToViewport` _returnvalue 0))

(event `Show/Hide Scope`
  (bind _scopewidget (`self.ScopeWidget`))
  (if (`self.Scope`)
    (set `self.Scope` false)
    (`/Engine/EditorBlueprintResources/StandardMacros.IsValid` _scopewidget
      (:`Is Valid`
        (`Widget.RemoveFromParent` _scopewidget)))
    (else
      (set `self.Scope` true)
      (bind _returnvalue (`|CreateWidget` "/Game/UserWidget/WBP_Scope.WBP_Scope_C"))
      (bind _output_get (set `self.ScopeWidget` _returnvalue))
      (`UserWidget.AddToViewport` _output_get 0))))

(fn `UserConstructionScript`)