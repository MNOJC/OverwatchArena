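; BP_StickyBomb is a timed bomb that homes onto a BP_Dummy and explodes shortly after spawning.
; A physics hit stops the cube simulating, while a dummy entering the sphere caches it and starts a timeline meant to lerp the cube onto it and attach.
; After a fixed delay from BeginPlay it spawns an explosion, triggers hard damage on any cached dummy, then removes itself.
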(event `self.ReceiveBeginPlay`
  (bind _as_bp_dummy (`self.As BP Dummy`))
  (`KismetSystemLibrary.Delay` 3.0)
  (`GameplayStatics.SpawnEmitterAtLocation` "/Game/StarterContent/Particles/P_Explosion.P_Explosion" (`SceneComponent.K2_GetComponentLocation` (`self.Cube`)))
  (`/Engine/EditorBlueprintResources/StandardMacros.IsValid` _as_bp_dummy
    (:`Is Valid`
      (`/Game/Blueprint/BP_Dummy.PlayHardDamage` _as_bp_dummy))
    (:`Is Not Valid`
      _))
  (`ActorComponent.K2_DestroyComponent` (`self.Cube`))
  (`KismetSystemLibrary.Delay` 0.5)
  (`self.K2_DestroyActor`))

(event `self.Cube.OnComponentHit`
  (params (HitComponent :type "PrimitiveComponent Object Reference") (OtherActor :type "Actor Object Reference") (OtherComp :type "PrimitiveComponent Object Reference") (NormalImpulse :type "Vector Structure") (Hit :type "HitResult Structure (by ref)"))
  (`PrimitiveComponent.SetSimulatePhysics` (`self.Cube`) false))

(event `self.Sphere.OnComponentBeginOverlap`
  (params (OverlappedComponent :type "PrimitiveComponent Object Reference") (OtherActor :type "Actor Object Reference") (OtherComp :type "PrimitiveComponent Object Reference") (OtherBodyIndex :type Integer) (bFromSweep :type Boolean) (SweepResult :type "HitResult Structure (by ref)"))
  (bind _asbp_dummy (cast `/Game/Blueprint/BP_Dummy` OtherActor))
  (set `self.As BP Dummy` _asbp_dummy)
  (`TimelineComponent.PlayFromStart` (`self.Timeline`)))

(fn `UserConstructionScript`)