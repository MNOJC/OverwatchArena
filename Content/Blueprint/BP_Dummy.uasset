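; BP_Dummy is a training dummy that plays damage reactions and can be launched into the air.
; Light and hard damage events play small and big hit animations on the skeletal mesh.
; Impulse enables physics and kicks the mesh upward.
; It then repeats a delayed, debug-drawn short trace along the actor's down axis from the mesh, disabling physics once something is hit.
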(event `PlayLightDamage`
  (`SkeletalMeshComponent.PlayAnimation` (`self.SkeletalMesh`) "/Game/Dummy/Animations/Training_Dummy_Anim_Damaged_Small.Training_Dummy_Anim_Damaged_Small" false))

(event `PlayHardDamage`
  (`SkeletalMeshComponent.PlayAnimation` (`self.SkeletalMesh`) "/Game/Dummy/Animations/Training_Dummy_Anim_Damaged_Big.Training_Dummy_Anim_Damaged_Big" false))

(event `Impulse`
  (bind _skeletalmesh (`self.SkeletalMesh`))
  (bind _returnvalue (`SceneComponent.K2_GetComponentLocation` (`self.SkeletalMesh`)))
  (`PrimitiveComponent.SetSimulatePhysics` _skeletalmesh true)
  (`PrimitiveComponent.AddImpulse` _skeletalmesh (0.0 0.0 99999.0) "None" false)
  (`KismetSystemLibrary.Delay` 4.0 :!label _label)
  (bind (_outhit _returnvalue_2) (`KismetSystemLibrary.LineTraceSingle` :`Start` _returnvalue :`End` (+ _returnvalue (* (* (`self.GetActorUpVector`) -1.0) 10)) :`TraceChannel` "TraceTypeQuery1" :`DrawDebugType` "ForDuration" :`DrawTime` 50.0))
  (if _returnvalue_2
    (`PrimitiveComponent.SetSimulatePhysics` _skeletalmesh false)
    (else
      (goto _label))))

(fn `UserConstructionScript`)