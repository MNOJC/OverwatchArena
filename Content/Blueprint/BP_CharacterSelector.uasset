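; BP_CharacterSelector is a world trigger that swaps the player's hero when a Player-tagged actor overlaps its box.
; It spawns the class chosen by CharactersSelected (only Genji and Widowmaker are wired) at that actor's location and rotation, possesses it and destroys the old actor.
; Its icon widget shows the selection and yaws toward the player each tick.
; SetActorToLook pushes the Player-tagged target to every selector after each swap.
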(event `self.ReceiveBeginPlay`
  (bind _returnvalue (`GameplayStatics.GetPlayerCharacter` 0))
  (bind _as_wbp_character_icon (`self.As WBP Character Icon`))
  (bind _aswbp_character_icon (cast `/Game/UserWidget/WBP_CharacterIcon` (`WidgetComponent.GetWidget` (`self.Widget`))))
  (set `self.As WBP Character Icon` _aswbp_character_icon)
  (bind _asbp_genji (cast `/Game/Characters/Genji/Blueprint/BP_Genji` _returnvalue)
    (:`then`
      (set `self.As BP Genji` _asbp_genji))
    (:`CastFailed`
      (bind _asbp_widowmaker (cast `/Game/Characters/Widowmaker/BP_Widowmaker` _returnvalue))
      (set `self.As BP Widowmaker` _asbp_widowmaker)))
  (`/Engine/EditorBlueprintResources/StandardMacros.IsValid` _as_wbp_character_icon
    (:`Is Valid`
      (`/Game/UserWidget/WBP_CharacterIcon.SetCharactersSelected` _as_wbp_character_icon (`self.CharactersSelected`))
      (`self.SetActorToLook`))))

(event `self.ReceiveTick`
  (params (DeltaSeconds :type "Float (single-precision)"))
  (bind _actortolook (`self.ActorToLook`))
  (bind (_returnvalue_roll _returnvalue_pitch _returnvalue_yaw) (`KismetMathLibrary.BreakRotator` (`KismetMathLibrary.FindLookAtRotation` (`self.K2_GetActorLocation`) (`self.K2_GetActorLocation` _actortolook))))
  (`/Engine/EditorBlueprintResources/StandardMacros.IsValid` _actortolook
    (:`Is Valid`
      (`SceneComponent.K2_SetRelativeRotation` (`self.Widget`) (`KismetMathLibrary.MakeRotator` 0.0 0.0 _returnvalue_yaw) false false))))

(event `self.Box.OnComponentBeginOverlap`
  (params (OverlappedComponent :type "PrimitiveComponent Object Reference") (OtherActor :type "Actor Object Reference") (OtherComp :type "PrimitiveComponent Object Reference") (OtherBodyIndex :type Integer) (bFromSweep :type Boolean) (SweepResult :type "HitResult Structure (by ref)"))
  (bind (_returnvalue_location _returnvalue_rotation) (`KismetMathLibrary.BreakTransform` (`self.GetTransform` OtherActor)))
  (if (`self.ActorHasTag` OtherActor "Player")
    (bind _returnvalue (`|SpawnActorFromClass` (select `/Game/Enums/eCharacterSelection` (`self.CharactersSelected`) :`NewEnumerator0` "/Game/Characters/Genji/Blueprint/BP_Genji.BP_Genji_C" :`NewEnumerator1` "/Game/Characters/Widowmaker/BP_Widowmaker.BP_Widowmaker_C" :!type "Actor Class Reference") (`KismetMathLibrary.MakeTransform` _returnvalue_location _returnvalue_rotation) "Undefined" "MultiplyWithRoot" null null))
    (`Controller.Possess` (`GameplayStatics.GetPlayerController` 0) (select `/Game/Enums/eCharacterSelection` (`self.CharactersSelected`) :`NewEnumerator0` (cast `/Game/Characters/Genji/Blueprint/BP_Genji` _returnvalue :!pure true) :`NewEnumerator1` (cast `/Game/Characters/Widowmaker/BP_Widowmaker` _returnvalue :!pure true) :!type "Pawn Object Reference"))
    (`self.SetActorToLook`)
    (`self.K2_DestroyActor` OtherActor)))

(fn `SetActorToLook`
  (bind _outactors (`GameplayStatics.GetAllActorsWithTag` "Player"))
  (for _array_element _outactors
    (set `self.ActorToLook` _array_element))
  (bind _outactors_2 (`GameplayStatics.GetAllActorsOfClass` "BP_CharacterSelector_C"))
  (for _array_element_2 _outactors_2
    (set `/Game/Blueprint/BP_CharacterSelector.ActorToLook` (`self.ActorToLook`) _array_element_2))
  (return))

(fn `UserConstructionScript`)