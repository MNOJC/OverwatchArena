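; BP_VenomMine is a timed mine actor that explodes three seconds after it begins play, with no damage logic in its graphs.
; Its Cube component stops simulating physics on a hit, freezing the mine where it lands.
; When the timer ends, it spawns an explosion emitter at the Cube's location, destroys the Cube, then destroys the actor after a short delay.
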(event `self.ReceiveBeginPlay`
  (`KismetSystemLibrary.Delay` 3.0)
  (`GameplayStatics.SpawnEmitterAtLocation` "/Game/StarterContent/Particles/P_Explosion.P_Explosion" (`SceneComponent.K2_GetComponentLocation` (`self.Cube`)))
  (`ActorComponent.K2_DestroyComponent` (`self.Cube`))
  (`KismetSystemLibrary.Delay` 0.5)
  (`self.K2_DestroyActor`))

(event `self.Cube.OnComponentHit`
  (params (HitComponent :type "PrimitiveComponent Object Reference") (OtherActor :type "Actor Object Reference") (OtherComp :type "PrimitiveComponent Object Reference") (NormalImpulse :type "Vector Structure") (Hit :type "HitResult Structure (by ref)"))
  (`PrimitiveComponent.SetSimulatePhysics` (`self.Cube`) false))

(fn `UserConstructionScript`)