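; Speed boost pickup that temporarily raises the speed of an overlapping actor tagged Player.
; Sphere overlap sends SpeedPickUpMessage through BPI_Character with a boosted value, then a lower one after a short delay.
; The static mesh is hidden with its collision off on pickup, and returns after a further delay so the pickup respawns.
; The Sphere's own collision is never explicitly disabled.
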(event `self.Sphere.OnComponentBeginOverlap`
  (params (OverlappedComponent :type "PrimitiveComponent Object Reference") (OtherActor :type "Actor Object Reference") (OtherComp :type "PrimitiveComponent Object Reference") (OtherBodyIndex :type Integer) (bFromSweep :type Boolean) (SweepResult :type "HitResult Structure (by ref)"))
  (bind _staticmesh (`self.StaticMesh`))
  (bind _staticmesh_2 (`self.StaticMesh`))
  (if (`self.ActorHasTag` OtherActor "Player")
    (if (`KismetSystemLibrary.DoesImplementInterface` OtherActor "/Game/Interfaces/BPI_Character.BPI_Character_C")
      (message `/Game/Interfaces/BPI_Character.SpeedPickUp` OtherActor 2000.0)
      (`SceneComponent.SetVisibility` _staticmesh_2 false true)
      (`PrimitiveComponent.SetCollisionEnabled` _staticmesh_2 "NoCollision")
      (`KismetSystemLibrary.Delay` 5.0)
      (message `/Game/Interfaces/BPI_Character.SpeedPickUp` OtherActor 600.0)
      (`KismetSystemLibrary.Delay` 15.0)
      (`SceneComponent.SetVisibility` _staticmesh true true)
      (`PrimitiveComponent.SetCollisionEnabled` _staticmesh "QueryAndPhysics"))))

(fn `UserConstructionScript`)